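; Enemy spawner actor that creates waves of BP_Enemy at its own transform, following the wave state held by a BP_EnemySpawn actor.
; A Delay on Tick acts as a four-second polling loop that looks up that actor each pass.
; When its wave counter differs from CurrentWave, it increments by one and reloads MinionCount.
; Otherwise it spawns and logs one enemy per pass until none remain.
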(event `self.ReceiveBeginPlay`
  (set `self.wave` 0)
  (set `self.minionsToCreate` 0))

(event `self.ReceiveTick`
  (params (DeltaSeconds :type "Float (single-precision)"))
  (`KismetSystemLibrary.Delay` 4.0)
  (bind _returnvalue (`GameplayStatics.GetActorOfClass` "/Game/BluePrints/BP_EnemySpawn.BP_EnemySpawn_C"))
  (if (!= (`self.wave`) (`/Game/BluePrints/BP_EnemySpawn.currentWave` _returnvalue))
    (set `self.wave` (+ (`self.wave`) 1))
    (set `self.minionsToCreate` (`/Game/BluePrints/BP_EnemySpawn.minionCount` _returnvalue))
    (elif (!= (`self.minionsToCreate`) 0)
      (`|SpawnActorFromClass` "/Game/BluePrints/BP_Enemy.BP_Enemy_C" (`self.GetTransform`) "Undefined" "MultiplyWithRoot" null null)
      (set `self.minionsToCreate` (- (`self.minionsToCreate`) 1))
      (`KismetSystemLibrary.LogString` "Enemy created"))))

(fn `UserConstructionScript`)