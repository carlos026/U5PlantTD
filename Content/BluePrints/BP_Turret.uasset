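; BP_Turret is a turret actor that automatically damages enemies within range of its Sphere component.
; Each Tick it queries the sphere for overlapping BP_Enemy actors and takes the last one in the array as TargetEnemy.
; It casts that target and subtracts a fixed amount directly from its Health every frame, so damage depends on frame rate, with no projectile or cooldown.
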(event `self.ReceiveTick`
  (params (DeltaSeconds :type "Float (single-precision)"))
  (bind _overlappingactors (`PrimitiveComponent.GetOverlappingActors` (`self.Sphere`) "/Game/BluePrints/BP_Enemy.BP_Enemy_C"))
  ;[1 1 1] Hit the target
  (if (> (`KismetArrayLibrary.Array_Length` _overlappingactors) 0)
    (bind _output_get (set `self.targetEnemy` (`|GetArrayItem` _overlappingactors (- (`KismetArrayLibrary.Array_Length` _overlappingactors) 1))))
    (bind _asbp_enemy (cast `/Game/BluePrints/BP_Enemy` _output_get))
    (set `/Game/BluePrints/BP_Enemy.health` (- (`/Game/BluePrints/BP_Enemy.health` _asbp_enemy) 1) _asbp_enemy)))

(fn `UserConstructionScript`)