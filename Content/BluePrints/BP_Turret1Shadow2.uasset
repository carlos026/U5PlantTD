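; BP_Turret1Shadow2 is a mouse-following placement preview, or shadow, for BP_Turret.
; Each tick it scales the deprojected mouse world direction into a fixed-height position, approximating the cursor's ground point without a trace.
; The swept move's return value sets IsDrag.
; It enables player input on BeginPlay, and a left click spawns a turret at its location when IsDrag is true, leaving the preview in place.
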(event `self.ReceiveBeginPlay`
  (`self.EnableInput` (`GameplayStatics.GetPlayerController` 0)))

(event `Key|LeftMouseButton`
  (params (Key :type "Key Structure"))
  (bind (_returnvalue_x _returnvalue_y) (`KismetMathLibrary.BreakVector` (`self.K2_GetActorLocation`)))
  (:`Pressed`
    (if (`self.isDrag`)
      (`|SpawnActorFromClass` "/Game/BluePrints/BP_Turret.BP_Turret_C" (`KismetMathLibrary.MakeTransform` (`KismetMathLibrary.MakeVector` _returnvalue_x _returnvalue_y 75.0)) "Undefined" "MultiplyWithRoot" null null))))

(event `self.ReceiveTick`
  (params (DeltaSeconds :type "Float (single-precision)"))
  (bind (_worldlocation _worlddirection) (`PlayerController.DeprojectMousePositionToWorld` (`GameplayStatics.GetPlayerController` 0)))
  (bind (_sweephitresult _returnvalue) (`self.K2_SetActorLocation` (`KismetMathLibrary.MakeVector` (- (* (.x _worlddirection) 3000.0) 300.0) (* (.y _worlddirection) 2500.0) 75.0) true true))
  (set `self.isDrag` _returnvalue))

(fn `UserConstructionScript`)