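; BP_EnemySpawn is a wave counter for enemy minions, though it contains no spawning logic yet.
; BeginPlay sets the minion count and starts at the first wave.
; Tick polls the count and, when it reaches zero, refills it and advances the wave, stopping after a fixed wave cap.
; Nothing in this graph decrements the count, and the overlap event is empty.
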(event `self.ReceiveBeginPlay`
  (set `self.minionCount` 10)
  (set `self.currentWave` 1))

(event `self.ReceiveTick`
  (params (DeltaSeconds :type "Float (single-precision)"))
  (if (< (`self.currentWave`) 11)
    (if (== (`self.minionCount`) 0)
      (set `self.minionCount` 10)
      (set `self.currentWave` (+ (`self.currentWave`) 1)))))

(fn `UserConstructionScript`)