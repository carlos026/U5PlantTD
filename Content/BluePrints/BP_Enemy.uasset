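; BP_Enemy is an enemy minion that travels through the level's TriggerBox actors as sequential waypoints.
; BeginPlay sets health, speed and the first target.
; Each Tick turns it toward the target and drives its ProjectileMovement velocity, advancing to the next box on arrival.
; It destroys itself after the last box, or at exactly zero health, where it also decrements BP_EnemySpawn's MinionCount.
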(event `self.ReceiveBeginPlay`
  ;[1 1 1] Set objective, life and speed.
  (set `self.health` 300)
  (set `self.speed` 70.0)
  (bind _outactors (`GameplayStatics.GetAllActorsOfClass` "/Script/Engine.TriggerBox"))
  (set `self.target` (`self.K2_GetActorLocation` (`|GetArrayItem` _outactors))))

(event `self.ReceiveTick`
  (params (DeltaSeconds :type "Float (single-precision)"))
  (bind (_returnvalue_roll _returnvalue_pitch _returnvalue_yaw) (`KismetMathLibrary.BreakRotator` (`self.K2_GetActorRotation`)))
  ;[1 1 1] Move to the objective, check current life and status (debuff).
  (if (== (`self.health`) 0)
    (bind _returnvalue (`GameplayStatics.GetActorOfClass` "/Game/BluePrints/BP_EnemySpawn.BP_EnemySpawn_C"))
    (set `/Game/BluePrints/BP_EnemySpawn.minionCount` (- (`/Game/BluePrints/BP_EnemySpawn.minionCount` _returnvalue) 1) _returnvalue)
    (`self.K2_DestroyActor`)
    (elif (== (`self.K2_GetActorLocation`) (`self.target`) :`ErrorTolerance` 1.0)
      (bind _result (`/Engine/EditorBlueprintResources/StandardMacros.IncrementInt` (`self.checkpoints`))
        (:`  `
          (bind _outactors (`GameplayStatics.GetAllActorsOfClass` "/Script/Engine.TriggerBox"))
          (if (== _result (`KismetArrayLibrary.Array_Length` _outactors))
            (`self.K2_DestroyActor`)
            (else
              (set `self.target` (`self.K2_GetActorLocation` (`|GetArrayItem` _outactors (`self.checkpoints`))))))))
      (else
        ;;[0.04065 1 0.3368] Move projectile to the target
        (`self.K2_SetActorRotation` (`KismetMathLibrary.FindLookAtRotation` (`self.K2_GetActorLocation`) (`self.target`)))
        (set `MovementComponent.Velocity` (* (`KismetMathLibrary.CreateVectorFromYawPitch` _returnvalue_yaw _returnvalue_pitch) (`self.speed`)) (`self.ProjectileMovement`))))))

(fn `UserConstructionScript`)